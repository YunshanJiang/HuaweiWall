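; MyIntroState is the intro state actor for an FSM, signalling MyFSMManager when the intro step is done.
; On BeginPlay it enables input for player 0 and prints a debug "Intro" message.
; Q plays a timeline that drives SetQRCodePos on the MainCanvas widget held by MyCharacter, then calls StateDone when finished.
; Key 1 calls StateDone immediately, skipping the animation.
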(event EventBeginPlay
  (Input|EnableInput (Game|GetPlayerController 0))
  (Development|PrintString "Intro"))

(event Collision|EventActorBeginOverlap
  (params (OtherActor :type Actor%20Object%20Reference)))

(event EventTick
  (params (DeltaSeconds :type Float%20%28single-precision%29)))

(event Input|KeyboardEvents|1
  (params (Key :type Key%20Structure :default "None"))
  (:Pressed
    (bind _returnvalue (Actor|GetActorOfClass "/Game/Blueprints/MyFSMManager.MyFSMManager_C"))
    (Default|StateDone _returnvalue)))

(event Input|KeyboardEvents|Q
  (params (Key :type Key%20Structure :default "None"))
  (:Pressed
    (bind _asmy_character (Utilities|Casting|CastToMyCharacter (Game|GetPlayerCharacter 0)))
    (bind _新建轨道_0 (Timeline|时间轴 PlayFromStart)
      (:Update
        (bind _asmain_canvas (Utilities|Casting|CastToMainCanvas (Variables|/Game/Blueprints/MyCharacter.MyCharacter_C|Getwidget _asmy_character)))
        (Default|SetQRCodePos _asmain_canvas _新建轨道_0))
      (:Finished
        (bind _returnvalue (Actor|GetActorOfClass "/Game/Blueprints/MyFSMManager.MyFSMManager_C"))
        (Default|StateDone _returnvalue)))))

(fn ConstructionScript)