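; MyFSMManager is a simple state machine manager actor that represents each state as a spawned actor.
; On BeginPlay it enables player input, spawns MyIntroState at the origin and tracks it in CurrentStateActor.
; Pressing Q destroys the current state actor and spawns MyInteractionState, though it sets the CurrentState variable to Intro.
; The 1 key only prints a debug greeting, and nothing switches back to the intro state.
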(event EventBeginPlay
  (Input|EnableInput (Game|GetPlayerController 0))
  (bind _returnvalue (Game|SpawnActorfromClass "/Game/Blueprints/MyIntroState.MyIntroState_C" (Math|Conversions|ToTransform(Vector) (Math|Vector|MakeVector 0.0 0.0 0.0)) "Undefined" "MultiplyWithRoot" 0 0))
  (Variables|Default|SetCurrentStateActor _returnvalue))

(event Collision|EventActorBeginOverlap
  (params (OtherActor :type Actor%20Object%20Reference)))

(event EventTick
  (params (DeltaSeconds :type Float%20%28single-precision%29)))

(event Input|KeyboardEvents|Q
  (params (Key :type Key%20Structure :default "None"))
  (:Pressed
    (Variables|Default|SetCurrentState "Intro")
    (Actor|DestroyActor (Variables|Default|GetCurrentStateActor))
    (bind _returnvalue (Game|SpawnActorfromClass "/Game/Blueprints/MyInteractionState.MyInteractionState_C" (Math|Conversions|ToTransform(Vector) (Math|Vector|MakeVector 0.0 0.0 0.0)) "Undefined" "MultiplyWithRoot" 0 0))
    (bind _output_get (Variables|Default|SetCurrentStateActor _returnvalue))))

(event Input|KeyboardEvents|1
  (params (Key :type Key%20Structure :default "None"))
  (:Pressed
    (Development|PrintString "Hello")))

(fn ConstructionScript)